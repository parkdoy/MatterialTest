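; BP_Cube is a clickable cube actor that changes color with each click and explodes once its counter fills up.
; Each click adds to Count, writes it to the X (red) channel of the material's Color parameter and plays a switch sound.
; The material update runs before the threshold check, which spawns an explosion emitter at the cube's location and destroys the actor.
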(event `self.Cube.OnClicked`
  (params (TouchedComponent :type "PrimitiveComponent Object Reference") (ButtonPressed :type "Key Structure"))
  (bind _output_get (set `self.Count` (+ (`self.Count`) 0.2)))
  ;[1 1 1] 분기문 전에 값을 줘야함
  (`MeshComponent.SetVectorParameterValueOnMaterials` (`self.Cube`) "Color" (`KismetMathLibrary.MakeVector` (`self.Count`)))
  (`GameplayStatics.PlaySound2D` "/Engine/VREditor/Sounds/UI/Flashlight_Switch.Flashlight_Switch" 1.0 1.0 0.0 null null)
  (if (>= _output_get 1.0)
    (`GameplayStatics.SpawnEmitterAtLocation` "/Game/StarterContent/Particles/P_Explosion.P_Explosion" (`SceneComponent.K2_GetComponentLocation` (`self.Cube`)))
    (`self.K2_DestroyActor`)))

(fn `UserConstructionScript`)